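; LevelStreamer is a trigger actor that moves the game to another level when the player character enters its box.
; On overlap it creates a loading widget, adds it to the viewport and waits briefly before opening LevelToStream by name.
; Despite the asset name, it uses a full OpenLevel call rather than level streaming, then removes the widget immediately after that call.
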(event OnComponentBeginOverlap(Box)
  (params (OverlappedComponent :type Primitive%20Component%20Object%20Reference) (OtherActor :type Actor%20Object%20Reference) (OtherComp :type Primitive%20Component%20Object%20Reference) (OtherBodyIndex :type Integer) (bFromSweep :type Boolean) (SweepResult :type Hit%20Result%20Structure%20%28by%20ref%29))
  (if (== OtherActor (Game|GetPlayerCharacter 0))
    (bind _returnvalue (UserInterface|CreateWidget "/Game/Widgets/LoadingWidget.LoadingWidget_C"))
    (bind _output_get (Variables|Default|SetLoad%20Widget _returnvalue))
    (UserInterface|Viewport|AddtoViewport _output_get 0)
    (Utilities|FlowControl|Delay 0.5)
    (Game|OpenLevel(byName) (Variables|Default|GetLevelToStream))
    (Widget|RemovefromParent (Variables|Default|GetLoad%20Widget))))

(fn ConstructionScript)